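; Prototype torch that casts a light beam and carries a rotating line-of-sight component for detecting spectres.
; Each tick, a camera-channel trace ignoring the player feeds hit or default distance into the beam's DistanceMax parameter.
; On begin play, TorchLOS starts tracing, mesh building and rotation, then is immediately deactivated.
; Its overlap event only prints a debug death message for spectres, and the distance-growth step adds zero.
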(event `self.ReceiveTick`
  (params (DeltaSeconds :type "Float (single-precision)"))
  (bind _lightbeam (`self.LightBeam`))
  (bind _distance (`self.Distance`))
  (bind _returnvalue (`SceneComponent.K2_GetComponentLocation` _lightbeam))
  (`|ExecutionSequence`
    (:`then_0`
      (bind _outhit (`KismetSystemLibrary.LineTraceSingle` _returnvalue (+ _returnvalue (* (`SceneComponent.GetForwardVector` _lightbeam) _distance)) "TraceTypeQuery2" false (`|MakeArray` (`self.TPS_Player`) :!type "Actor Object Reference") "ForOneFrame"))
      (bind (_bblockinghit _binitialoverlap _time _distance_2) (`GameplayStatics.BreakHitResult` _outhit))
      (if _bblockinghit
        (`FXSystemComponent.SetFloatParameter` (`self.LightBeam`) "DistanceMax" _distance_2)
        (else
          (`FXSystemComponent.SetFloatParameter` (`self.LightBeam`) "DistanceMax" _distance))))
    (:`then_1`
      (if (< (`self.Distance`) 5000.0)
        (set `self.Distance` (+ (`self.Distance`) (* 0.0 2000.0)))))))

(event `self.ReceiveBeginPlay`
  (bind _torchlos (`self.TorchLOS`))
  (`|ExecutionSequence`
    (:`then_0`
      (`LineOfSightComponent.StartLineTrace` _torchlos "TraceTypeQuery1" 60)
      (`LineOfSightComponent.StartBuildMesh` _torchlos)
      (`LineOfSightComponent.StartRotateInRangeAxis` _torchlos "X" 90.0 15.0 "Relative_Rotation" false)
      (`ActorComponent.Deactivate` _torchlos))
    (:`then_1`
      (bind _asbp_third_person_character (cast `/Game/ThirdPerson/Blueprints/BP_ThirdPersonCharacter` (`GameplayStatics.GetPlayerCharacter` 0)))
      (set `self.TPS_Player` _asbp_third_person_character))))

(event `self.TorchLOS.BeginOverlap`
  (params (Hit :type "HitResult Structure (by ref)"))
  (cast `/Game/Game/PlaceHolder/Blueprints/BP_SpectreTest` (`.HitActor` (`GameplayStatics.BreakHitResult` Hit)))
  (`KismetSystemLibrary.PrintString` "TIE MORT" true true (struct :`R` 0.427083 :`G` 0.029549 :`A` 1.0)))

(fn `UserConstructionScript`)