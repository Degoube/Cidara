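; BP_LightRuneBeam is a placeholder light rune beam actor driven by the LightBeam Niagara effect, which it tints on BeginPlay.
; Each tick it line traces on the Camera channel along the beam's forward vector, with debug drawing on.
; The hit distance, or a default maximum on a miss, sets the effect's DistanceMax parameter.
; A capped Distance increment sets trace reach, but currently adds zero.
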(event `self.ReceiveBeginPlay`
  (`FXSystemComponent.SetColorParameter` (`self.LightBeam`) "LinearColor" (struct :`R` 100.0 :`G` 100.956123 :`B` 10.104167 :`A` 1.0)))

(event `self.ReceiveTick`
  (params (DeltaSeconds :type "Float (single-precision)"))
  (bind _lightbeam (`self.LightBeam`))
  (bind _returnvalue (`SceneComponent.K2_GetComponentLocation` _lightbeam))
  (bind _returnvalue_2 (+ _returnvalue (* (`SceneComponent.GetForwardVector` _lightbeam) (`self.Distance`))))
  (`|ExecutionSequence`
    (:`then_0`
      (set `self.TraceEnd` _returnvalue_2)
      (bind _outhit (`KismetSystemLibrary.LineTraceSingle` :`Start` _returnvalue :`End` _returnvalue_2 :`TraceChannel` "TraceTypeQuery2" :`DrawDebugType` "ForOneFrame"))
      (bind (_bblockinghit _binitialoverlap _time _distance) (`GameplayStatics.BreakHitResult` _outhit))
      (if _bblockinghit
        (`FXSystemComponent.SetFloatParameter` (`self.LightBeam`) "DistanceMax" _distance)
        (else
          (`FXSystemComponent.SetFloatParameter` (`self.LightBeam`) "DistanceMax" (`self.DistanceMaxNiagara`)))))
    (:`then_1`
      (if (< (`self.Distance`) 5000.0)
        (set `self.Distance` (+ (`self.Distance`) (* 0.0 2000.0)))))))

(fn `UserConstructionScript`)