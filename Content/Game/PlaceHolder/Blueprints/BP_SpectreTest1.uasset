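; Test Spectre character that moves and climbs walls through externally triggered events, oriented by the first-person character's active camera.
; MoveSpectre aligns it to Camera1 or Camera2's stored forward vector, then applies movement, snapping the mesh by input direction when not climbing.
; SpectreGrimpe starts climbing in Flying mode when a short debug-drawn trace hits.
; Tick keeps it facing the wall; its StopClimbing branch is unreachable because the condition is hardcoded true.
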(event `self.ReceiveBeginPlay`
  (`|ExecutionSequence`
    (:`then_0`
      (bind _asbp_first_person_character (cast `/Game/Game/Characters/FirstPerson/Blueprints/BP_FirstPersonCharacter` (`GameplayStatics.GetPlayerCharacter` 0)))
      (set `self.FPSCharac` _asbp_first_person_character))))

(event `MoveSpectre`
  (params (X :type "Float (double-precision)") (Y :type "Float (double-precision)"))
  (bind (_returnvalue_roll _returnvalue_pitch _returnvalue_yaw) (`KismetMathLibrary.BreakRotator` (`self.GetControlRotation`)))
  (bind _returnvalue (`self.GetActorRightVector`))
  (bind _fpscharac (`self.FPSCharac`))
  (bind _mesh (`self.Mesh`))
  ;[1 1 1] Permet a Spectre de bouger
  (if (`/Game/Game/Characters/FirstPerson/Blueprints/BP_FirstPersonCharacter.Camera1` _fpscharac)
    (`self.K2_SetActorRotation` (`KismetMathLibrary.Conv_VectorToRotator` (`/Game/Game/Characters/FirstPerson/Blueprints/BP_FirstPersonCharacter.FwdVectorCam1` _fpscharac)))
    (if (`self.IsClimbing?`) :!label _label
      ;;[0.3333 0.3333 0.3333] Climb
      (`self.AddMovementInput` _returnvalue X)
      (else
        (`self.AddMovementInput` _returnvalue X)))
    (if (`self.IsClimbing?`)
      (`self.AddMovementInput` (`KismetMathLibrary.GetUpVector` (`KismetMathLibrary.MakeRotator` 0.0 0.0 _returnvalue_yaw)) Y)
      (else
        (`self.AddMovementInput` (`self.GetActorForwardVector`) Y)
        ;[1 1 1] tourner spectre dans la direction ou elle se dirige
        (`|ExecutionSequence`
          (:`then_0`
            (if (> Y 0.1)
              (`SceneComponent.K2_SetWorldRotation` _mesh (`KismetMathLibrary.Conv_VectorToRotator` (`KismetMathLibrary.Vector_SlerpNormals` (0.0 0.0 0.0) (`KismetMathLibrary.GetRightVector` (struct)))) false false)))
          (:`then_1`
            (if (< Y -0.1)
              (`SceneComponent.K2_SetWorldRotation` _mesh (struct :`Yaw` -180.0) false false)))
          (:`then_2`
            (if (> X 0.1)
              (`SceneComponent.K2_SetWorldRotation` _mesh (struct :`Yaw` 90.0) false false)))
          (:`then_3`
            (if (< X -0.1)
              (`SceneComponent.K2_SetWorldRotation` _mesh (struct :`Yaw` -90.0) false false))))))
    (elif (`/Game/Game/Characters/FirstPerson/Blueprints/BP_FirstPersonCharacter.Camera2` _fpscharac)
      (`self.K2_SetActorRotation` (`KismetMathLibrary.Conv_VectorToRotator` (`/Game/Game/Characters/FirstPerson/Blueprints/BP_FirstPersonCharacter.FwdVectorCam2` _fpscharac)))
      (goto _label))))

(event `StopClimbing`
  ;[0.4323 0.4323 0.4323] Stop climbing
  (set `self.IsClimbing?` false)
  (`CharacterMovementComponent.SetMovementMode` (`self.CharacterMovement`) "MOVE_Falling" 0))

(event `SpectreGrimpe`
  (bind (_returnvalue_roll _returnvalue_pitch) (`KismetMathLibrary.BreakRotator` (`self.K2_GetActorRotation`)))
  ;[0.4323 0.4323 0.4323] Faire escalader Spectre
  (bind (_outhit _hashit_) (`self.ClimbingLineTrace`))
  (if _hashit_
    (set `self.IsClimbing?` true)
    (`CharacterMovementComponent.SetMovementMode` (`self.CharacterMovement`) "MOVE_Flying" 0)
    (bind (_returnvalue_roll_2 _returnvalue_pitch_2 _returnvalue_yaw) (`KismetMathLibrary.BreakRotator` (`KismetMathLibrary.MakeRotFromX` (`.Normal` (`GameplayStatics.BreakHitResult` _outhit)))))
    ;;[1 1 1] Faire en sorte que le personnage regarde le mur
    (`self.K2_SetActorRotation` (`KismetMathLibrary.MakeRotator` _returnvalue_roll _returnvalue_pitch (+ _returnvalue_yaw 180.0)))))

(event `self.ReceiveTick`
  (params (DeltaSeconds :type "Float (single-precision)"))
  (bind (_returnvalue_roll _returnvalue_pitch) (`KismetMathLibrary.BreakRotator` (`self.K2_GetActorRotation`)))
  ;[0.4323 0.4323 0.4323] Boucle d'escalade
  (if (`self.IsClimbing?`)
    (bind _outhit (`self.ClimbingLineTrace`))
    (if true
      (bind (_returnvalue_roll_2 _returnvalue_pitch_2 _returnvalue_yaw) (`KismetMathLibrary.BreakRotator` (`KismetMathLibrary.MakeRotFromX` (`.Normal` (`GameplayStatics.BreakHitResult` _outhit)))))
      (`self.K2_SetActorRotation` (`KismetMathLibrary.MakeRotator` _returnvalue_roll _returnvalue_pitch (+ _returnvalue_yaw 180.0)))
      (else
        (`self.StopClimbing`)))))

(fn `ClimbingLineTrace`
  (returns (OutHit :type "HitResult Structure") (`HasHit?` :type Boolean))
  (bind _returnvalue (`self.K2_GetActorLocation`))
  (bind (_outhit _returnvalue_2) (`KismetSystemLibrary.LineTraceSingle` :`Start` _returnvalue :`End` (+ _returnvalue (* -100.0 (`SceneComponent.GetForwardVector` (`self.Mesh`)))) :`TraceChannel` "TraceTypeQuery1" :`DrawDebugType` "ForDuration" :`DrawTime` 2.0))
  (return _outhit _returnvalue_2))

(fn `UserConstructionScript`)